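; EnemyBulletBp is an enemy bullet projectile, filed under the assault rifle, for a 2D side-scroller.
; Each Tick rotates the scene root to face the ProjectileMovement velocity, then feeds a Delay that destroys the bullet, acting as a short lifetime timer from the first frame.
; Overlapping the 2D_Sidescroller_BluePrint actor destroys it after a brief delay; no damage is applied here.
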(event `self.ReceiveActorBeginOverlap`
  (params (OtherActor :type "Actor Object Reference"))
  (cast `/Game/2-Point-5-D/2D_Sidescroller_BluePrint` OtherActor)
  (`KismetSystemLibrary.Delay` 0.05)
  (`self.K2_DestroyActor`))

(event `self.ReceiveTick`
  (params (DeltaSeconds :type "Float (single-precision)"))
  (bind _returnvalue (`self.K2_GetActorLocation`))
  (`SceneComponent.K2_SetWorldRotation` (`self.DefaultSceneRoot`) (`KismetMathLibrary.FindLookAtRotation` _returnvalue (+ _returnvalue (`MovementComponent.Velocity` (`self.ProjectileMovement`)))) false false)
  (`KismetSystemLibrary.Delay` 0.75)
  (`self.K2_DestroyActor`))

(fn `UserConstructionScript`)