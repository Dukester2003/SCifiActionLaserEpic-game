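; Rooftop ladder actor that marks where the side-scroller player character can climb.
; When the character enters its Box trigger, it casts to the player's animation Blueprint and sets ShouldClimb to true, then clears it on exit.
; The ladder only toggles that animation flag and contains no movement logic of its own.
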(event `self.Box.OnComponentBeginOverlap`
  (params (OverlappedComponent :type "PrimitiveComponent Object Reference") (OtherActor :type "Actor Object Reference") (OtherComp :type "PrimitiveComponent Object Reference") (OtherBodyIndex :type Integer) (bFromSweep :type Boolean) (SweepResult :type "HitResult Structure (by ref)"))
  (bind _as2d_sidescroller_blue_print (cast `/Game/2-Point-5-D/2D_Sidescroller_BluePrint` OtherActor))
  (bind _asplayer_anim_bp (cast `/Game/Characters/Player/Animations/PlayerAnimBP` (`SkeletalMeshComponent.GetAnimInstance` (`Character.Mesh` _as2d_sidescroller_blue_print))))
  (set `/Game/Characters/Player/Animations/PlayerAnimBP.Should Climb` true _asplayer_anim_bp))

(event `self.Box.OnComponentEndOverlap`
  (params (OverlappedComponent :type "PrimitiveComponent Object Reference") (OtherActor :type "Actor Object Reference") (OtherComp :type "PrimitiveComponent Object Reference") (OtherBodyIndex :type Integer))
  (bind _as2d_sidescroller_blue_print (cast `/Game/2-Point-5-D/2D_Sidescroller_BluePrint` OtherActor))
  (bind _asplayer_anim_bp (cast `/Game/Characters/Player/Animations/PlayerAnimBP` (`SkeletalMeshComponent.GetAnimInstance` (`Character.Mesh` _as2d_sidescroller_blue_print))))
  (set `/Game/Characters/Player/Animations/PlayerAnimBP.Should Climb` false _asplayer_anim_bp))

(fn `UserConstructionScript`)